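; BP_PauseMenu is an actor that hosts the pause menu in a widget component and forwards menu selection input to it.
; On BeginPlay it casts the component's user widget to WB_PauseMenu and stores the reference.
; The MenuSelect event calls NextButton on that widget, using an IsClicked flag and a short delay to debounce repeated triggers.
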(event `self.ReceiveBeginPlay`
  (bind _aswb_pause_menu (cast `/Game/GMC/WB_PauseMenu` (`WidgetComponent.GetUserWidgetObject` (`self.Widget`))))
  (set `self.PauseMenu` _aswb_pause_menu))

(event `MenuSelect`
  (if (not (`self.Is Clicked`))
    (set `self.Is Clicked` true)
    (`/Game/GMC/WB_PauseMenu.NextButton` (`self.PauseMenu`))
    (`KismetSystemLibrary.Delay` 0.2)
    (set `self.Is Clicked` false)))

(fn `UserConstructionScript`)