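; BP_TextTyping shows a hardcoded test string in its widget as a typewriter effect, starting at BeginPlay.
; A delayed loop increments an index and passes a growing left substring to WBP_TextTyping's SettingText, one character per step.
; The TypingStart event and Delay function are empty stubs, and CurString is only initialized.
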(event `TypingStart`)

(event `self.ReceiveBeginPlay`
  (set `self.TargetString` "testtesttesttesttesttesttesttesttest")
  (set `self.CurString` "")
  (set `self.index` 0)
  (`/Game/GMC/BPM.ForLoopWithDelay` 0 (`KismetStringLibrary.Len` (`self.TargetString`)) 1
    (:`LoopBody`
      (bind _aswbp_text_typing (cast `/Game/GMC/WBP_TextTyping` (`WidgetComponent.GetUserWidgetObject` (`self.Widget`))))
      (set `self.index` (+ (`self.index`) 1))
      (`/Game/GMC/WBP_TextTyping.SettingText` _aswbp_text_typing (`KismetStringLibrary.Left` (`self.TargetString`) (`self.index`))))))

(fn `Delay`)

(fn `UserConstructionScript`)