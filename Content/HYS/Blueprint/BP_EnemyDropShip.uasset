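; Enemy drop ship actor that deploys BP_Enemy_Ranged units while flying, then removes itself.
; After BeginPlay, a delayed loop spawns one unit per second at SpawnPoint until SpawnMaxNum, then sets IsSpawnEnd and destroys the ship ten seconds later.
; Tick moves the Ship component along local -Y and plays the ShipMovement timeline, whose vector track drives incremental pitch, adding roll once spawning ends.
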(event `SpawnUnit`
  ;[0.349 0.349 0.349 1 30] SpawnUnit
  (if (>= (`self.SpawnCurrentNum`) (`self.SpawnMaxNum`)) :!label _label
    (set `self.isSpawnEnd` true)
    (`KismetSystemLibrary.Delay` 10.0)
    (`self.K2_DestroyActor`)
    (else
      (`KismetSystemLibrary.Delay` 1.0)
      (`|SpawnActorFromClass` "/Game/Drkong/Enemy/BP_Enemy_Ranged.BP_Enemy_Ranged_C" (`SceneComponent.K2_GetComponentToWorld` (`self.SpawnPoint`)) "Undefined" "MultiplyWithRoot" null null)
      (set `self.SpawnCurrentNum` (+ (`self.SpawnCurrentNum`) 1))
      (goto _label))))

(event `self.ReceiveBeginPlay`
  (`KismetSystemLibrary.Delay` 1.0)
  (`self.SpawnUnit`))

(event `self.ReceiveTick`
  (params (DeltaSeconds :type "Float (single-precision)"))
  (`SceneComponent.K2_AddLocalOffset` (`self.Ship`) (0.0 -30.0 0.0) false false)
  (bind (_direction _vectorx) (`Timeline|ShipMovement`)
    (:`Update`
      (`SceneComponent.K2_AddLocalRotation` (`self.Ship`) (`KismetMathLibrary.MakeRotator` 0.0 (.x _vectorx)) false false)
      (if (`self.isSpawnEnd`)
        (`SceneComponent.K2_AddLocalRotation` (`self.Ship`) (`KismetMathLibrary.MakeRotator` (.y _vectorx)) false false)))))

(fn `UserConstructionScript`)