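; Base Blueprint for over-time area-of-effect actors, built on a parent class that supplies the Trigger event.
; Trigger runs the parent logic, then starts a looping timer at SpawnInterval and a one-shot timer for the Dureation variable.
; The events those timers fire are not defined in this graph.
; BeginPlay, overlap and Tick are inactive, and the construction script only calls its parent.
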(event `self.Trigger`
  (`parent.Trigger`)
  (`|ExecutionSequence`
    (:`then_0`
      (`KismetSystemLibrary.K2_SetTimerDelegate` (`|CreateDelegate` :!event `SpawnAOESphere`) (`self.SpawnInterval`) true))
    (:`then_1`
      (`KismetSystemLibrary.K2_SetTimerDelegate` (`|CreateDelegate` :!event `K2_DestroyActor`) (`self.Dureation`)))))

(fn `UserConstructionScript`
  (`parent.UserConstructionScript`))