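; Area-of-effect boom attack actor that calls Trigger 0.2 seconds after BeginPlay, with Trigger defined outside this graph.
; MoveTOFloor snaps the actor to a Visibility trace hit from AttackTarget, with the trace end computed by multiplying the target's location rather than offsetting it downward.
; Its only call, along with the BP_BoomWarning spawn and cleanup nodes, is disconnected and never runs.
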(event `self.ReceiveBeginPlay`
  (`parent.ReceiveBeginPlay`)
  (`KismetSystemLibrary.Delay` 0.2)
  (`self.Trigger`))

(event `MoveTOFloor`
  (bind _attacktarget (`self.AttackTarget`)
    (:`then`
      (bind _returnvalue (`self.K2_GetActorLocation` _attacktarget))
      (bind (_outhit _returnvalue_2) (`KismetSystemLibrary.LineTraceSingle` _returnvalue (* _returnvalue (0.0 0.0 -1000.0)) "TraceTypeQuery1" false (`|MakeArray` _attacktarget)))
      (if _returnvalue_2
        (`self.K2_SetActorLocation` (`.Location` (`GameplayStatics.BreakHitResult` _outhit)))))
    (:`else`)))

(fn `UserConstructionScript`
  (`parent.UserConstructionScript`))