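; BP_Vship is a ship actor that travels along a spline path when play begins.
; BeginPlay finds the BP_SplinePath actor, then MoveObject plays a timeline scaled by TimeToCompleteInSeconds, mapping its track to distance along the spline.
; Each update takes only the location from the spline transform.
; Unconnected leftover logic covers VR pawn attachment, tower-to-tower teleporting and a roll timeline, and MoveTower2 is empty.
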(event `Move Object`
  (`TimelineComponent.SetPlayRate` (`self.Move Object T`) (/ 1.0 (`self.Time To Complete(in Seconds)`)))
  (bind (_direction _move_track) (`Timeline|Move Object T`)
    (:`Update`
      (bind _returnvalue_location (`KismetMathLibrary.BreakTransform` (`SplineComponent.GetTransformAtDistanceAlongSpline` (`/Game/jihoon/BP_SplinePath.Spline` (`self.Spline Ref`)) (`KismetMathLibrary.Lerp` 0.0 (`SplineComponent.GetSplineLength` (`/Game/jihoon/BP_SplinePath.Spline` (`self.Spline Ref`))) _move_track) "World" false)))
      (`self.K2_SetActorTransform` (`KismetMathLibrary.MakeTransform` _returnvalue_location)))))

(event `self.ReceiveBeginPlay`
  (bind _returnvalue (`GameplayStatics.GetActorOfClass` "/Game/jihoon/BP_SplinePath.BP_SplinePath_C"))
  (set `self.Spline Ref` _returnvalue)
  (`self.Move Object`))

(event `MoveTower2`)

(fn `UserConstructionScript`)