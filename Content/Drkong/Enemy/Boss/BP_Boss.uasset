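; Flying boss enemy that bobs on a timeline while drifting forward, with machine-gun and rocket attacks.
; DefaultAttack aims four cannons at the target and fires bullets, two with random spread.
; SkilAttack places a warning marker at the target, launches a homing rocket at it, then spawns an AOE blast on impact that damages other teams.
; Death triggers an explosion, defeat sound and DestroyActor, followed by a delayed QuitGame call.
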(event `self.ReceiveBeginPlay`
  ;[0.3073 0.3073 0.3073 1 30] Floating
  (`parent.ReceiveBeginPlay`)
  (bind (_direction _dumping) (`Timeline|타임라인_2`)
    (:`Update`
      (`self.K2_AddActorLocalOffset` (`KismetMathLibrary.MakeVector` 0.0 0.0 _dumping))
      (`self.K2_AddActorLocalOffset` (10.0 0.0 0.0)))))

(event `/Game/Drkong/Enemy/AI/BPI_EnemyAI.SkilAttack`
  (params (AttackTarget :type "Actor Object Reference"))
  ;[0.1615 0.1615 0.1615 1 30] Spawn Rocket and AOE Attack(add Warning)
  (set `self.Attack Target` AttackTarget)
  (`self.Warnning`)
  (`KismetSystemLibrary.Delay` 0.2)
  (bind _returnvalue (`|SpawnActorFromClass` "/Game/Drkong/Projectiles/BP_ProjectileRocket.BP_ProjectileRocket_C" (`SceneComponent.K2_GetComponentToWorld` (`self.RocketLaunchedPoint`)) "Undefined" "MultiplyWithRoot" null 3000.0 0.0 (`self.BoomWarning`) true null))
  (add `/Game/Drkong/Projectiles/BP_Projectile_Base.OnProjectileImpact` _returnvalue (delegate `OnProjectileImpact_이벤트`)))

(event `OnProjectileImpact_이벤트`
  (params (OtherActor :type "Actor Object Reference") (Hit :type "HitResult Structure"))
  ;[0.1615 0.1615 0.1615 1 30] Spawn Rocket and AOE Attack(add Warning)
  (`/Engine/EditorBlueprintResources/StandardMacros.IsValid` (`self.Attack Target`)
    (:`Is Valid`
      (bind _returnvalue (`|SpawnActorFromClass` "/Game/HYS/AOE/BP_AOE_Boom.BP_AOE_Boom_C" (`self.GetTransform` (`self.BoomWarning`)) "Undefined" "MultiplyWithRoot" null 0.0 null false false null))
      (add `/Game/HYS/AOE/BP_AOE_Base.OnAOEOverlapActor` _returnvalue (delegate `OnAOEOverlapActor_이벤트`)))))

(event `OnAOEOverlapActor_이벤트`
  (params (Actor :type "Actor Object Reference"))
  ;[0.1615 0.1615 0.1615 1 30] Spawn Rocket and AOE Attack(add Warning)
  (bind _team_number (message `/Game/Drkong/DamageSystem/BPI_Damageable.GetTeamNumber` Actor))
  (if (!= _team_number (`self.TeamNumber`))
    (message `/Game/Drkong/DamageSystem/BPI_Damageable.TakeDamage` Actor (make `/Game/Drkong/DamageSystem/S_DamageInfo` 40.0 "NewEnumerator3" "NewEnumerator1"))))

(event `Warnning`
  ;[0.2552 0.2552 0.2552 1 30] Warnning
  (bind _returnvalue (`|SpawnActorFromClass` "/Game/HYS/Effect/BP_BoomWarning.BP_BoomWarning_C" (`self.GetTransform` (`self.Attack Target`)) "Undefined" "MultiplyWithRoot" null null))
  (bind _output_get (set `self.BoomWarning` _returnvalue))
  (bind _returnvalue_2 (`self.K2_GetActorLocation` _output_get))
  (bind (_outhit _returnvalue_3) (`KismetSystemLibrary.LineTraceSingle` _returnvalue_2 (* _returnvalue_2 (0.0 0.0 -1000.0)) "TraceTypeQuery1" false (`|MakeArray` _output_get :!type "Actor Object Reference")))
  (if _returnvalue_3
    (`self.K2_SetActorLocation` (`self.BoomWarning`) (`.Location` (`GameplayStatics.BreakHitResult` _outhit)) false false)))

(event `/Game/Drkong/Enemy/AI/BPI_EnemyAI.DefaultAttack`
  (params (AttackTarget :type "Actor Object Reference"))
  (bind _returnvalue (`self.K2_GetActorLocation` AttackTarget))
  (bind _returnvalue_2 (`self.K2_GetActorLocation` AttackTarget))
  (bind _returnvalue_3 (`KismetMathLibrary.MakeRotator` (`KismetMathLibrary.RandomFloatInRange` -3.0 3.0) (`KismetMathLibrary.RandomFloatInRange` -3.0 3.0) (`KismetMathLibrary.RandomFloatInRange` -3.0 3.0)))
  (bind _returnvalue_4 (`KismetMathLibrary.FindLookAtRotation` (`SceneComponent.K2_GetComponentLocation` (`self.CanonRay2`)) _returnvalue))
  (bind _returnvalue_5 (`KismetMathLibrary.FindLookAtRotation` (`SceneComponent.K2_GetComponentLocation` (`self.CanonRay1`)) _returnvalue))
  (bind _returnvalue_6 (`KismetMathLibrary.FindLookAtRotation` (`SceneComponent.K2_GetComponentLocation` (`self.CanonRay4`)) _returnvalue_2))
  (bind _returnvalue_7 (`KismetMathLibrary.FindLookAtRotation` (`SceneComponent.K2_GetComponentLocation` (`self.CanonRay3`)) _returnvalue_2))
  ;[0.2396 0.2396 0.2396 1 30] Machine Gun
  (`SceneComponent.K2_SetWorldRotation` (`self.CanonRay3`) _returnvalue_7 false false)
  (`SceneComponent.K2_SetWorldRotation` (`self.CanonRay4`) _returnvalue_6 false false)
  (`SceneComponent.K2_SetWorldRotation` (`self.CanonRay2`) _returnvalue_4 false false)
  (`SceneComponent.K2_SetWorldRotation` (`self.CanonRay1`) _returnvalue_5 false false)
  (bind _returnvalue_8 (`|SpawnActorFromClass` "/Game/Drkong/Projectiles/BP_ProjectileBullet_Boss.BP_ProjectileBullet_Boss_C" (`KismetMathLibrary.MakeTransform` (`SceneComponent.K2_GetComponentLocation` (`self.ProjectileLaunchPoint2`)) (`KismetMathLibrary.ComposeRotators` _returnvalue_4 _returnvalue_3)) "Undefined" "MultiplyWithRoot" null 6000.0 0.0 null false null))
  (bind _returnvalue_9 (`|SpawnActorFromClass` "/Game/Drkong/Projectiles/BP_ProjectileBullet_Boss.BP_ProjectileBullet_Boss_C" (`KismetMathLibrary.MakeTransform` (`SceneComponent.K2_GetComponentLocation` (`self.ProjectileLaunchPoint1`)) (`KismetMathLibrary.ComposeRotators` _returnvalue_5 _returnvalue_3)) "Undefined" "MultiplyWithRoot" null 6000.0 0.0 null false null))
  (bind _returnvalue_10 (`|SpawnActorFromClass` "/Game/Drkong/Projectiles/BP_ProjectileBullet_Boss.BP_ProjectileBullet_Boss_C" (`KismetMathLibrary.MakeTransform` (`SceneComponent.K2_GetComponentLocation` (`self.ProjectileLaunchPoint3`)) _returnvalue_7) "Undefined" "MultiplyWithRoot" null 6000.0 0.0 null false null))
  (bind _returnvalue_11 (`|SpawnActorFromClass` "/Game/Drkong/Projectiles/BP_ProjectileBullet_Boss.BP_ProjectileBullet_Boss_C" (`KismetMathLibrary.MakeTransform` (`SceneComponent.K2_GetComponentLocation` (`self.ProjectileLaunchPoint4`)) _returnvalue_6) "Undefined" "MultiplyWithRoot" null 6000.0 0.0 null false null))
  (add `/Game/Drkong/Projectiles/BP_Projectile_Base.OnProjectileImpact` _returnvalue_8 (delegate `ProjectileDamage`))
  (add `/Game/Drkong/Projectiles/BP_Projectile_Base.OnProjectileImpact` _returnvalue_9 (delegate `ProjectileDamage`))
  (add `/Game/Drkong/Projectiles/BP_Projectile_Base.OnProjectileImpact` _returnvalue_11 (delegate `ProjectileDamage`))
  (add `/Game/Drkong/Projectiles/BP_Projectile_Base.OnProjectileImpact` _returnvalue_10 (delegate `ProjectileDamage`))
  (`PrimitiveComponent.IgnoreActorWhenMoving` (`self.ProjectileLaunchPoint1`) null false)
  (`PrimitiveComponent.IgnoreActorWhenMoving` (`self.ProjectileLaunchPoint2`) null false))

(event `ProjectileDamage`
  (params (OtherActor :type "Actor Object Reference") (Hit :type "HitResult Structure"))
  ;[0.2396 0.2396 0.2396 1 30] Machine Gun
  (message `/Game/Drkong/DamageSystem/BPI_Damageable.TakeDamage` OtherActor (make `/Game/Drkong/DamageSystem/S_DamageInfo` 5.0)))

(event `self.BPC_DamageSystem.OnDeath`
  (`GameplayStatics.SpawnEmitterAtLocation` "/Game/MilitaryWeapDark/FX/P_RocketLauncher_Explosion_01.P_RocketLauncher_Explosion_01" (`self.K2_GetActorLocation`) (struct) (30.0 30.0 30.0))
  (`GameplayStatics.PlaySound2D` "/Game/HYS/Sound/BossDefeat.BossDefeat" 1.0 1.0 0.0 null null)
  (`self.K2_DestroyActor`)
  (`KismetSystemLibrary.Delay` 3.0)
  (`KismetSystemLibrary.QuitGame` null "Quit"))

(fn `GetIdealRange`
  (returns (AttackRadius :type "Float (double-precision)"))
  (return 30000.0))

(fn `GetTeamNumber`
  (returns (`Team Number` :type Integer))
  (return 1))

(fn `UserConstructionScript`
  (`parent.UserConstructionScript`))