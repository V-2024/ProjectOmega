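; Base enemy character that delegates health and damage to BPC_DamageSystem and shows a health bar widget.
; On BeginPlay it caches its AIC_Enemy_Base controller, creates the health bar and binds the damage system's death event.
; Death ragdolls the mesh, stops AI logic, sets the dead state, hides the bar and destroys the actor after a delay.
; Speed states set walk speed; Heal and IsDead are stubs returning constants.
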(event `self.ReceiveBeginPlay`
  (bind _asaic_enemy_base (cast `/Game/Drkong/Enemy/AI/AIC_Enemy_Base` (`AIBlueprintHelperLibrary.GetAIController` self)))
  (set `self.AICEnemyBase` _asaic_enemy_base)
  (bind _returnvalue (`|CreateWidget` "/Game/Drkong/DamageSystem/W_HealthBar.W_HealthBar_C" null self))
  (`WidgetComponent.SetWidget` (`self.HealthBar`) _returnvalue)
  (add `/Game/Drkong/DamageSystem/BPC_DamageSystem.OnDeath` (`self.BPC_DamageSystem`) (`|CreateDelegate` :!event `OnDeath_Event`)))

(event `OnDeath_Event`
  (bind _mesh (`self.Mesh`))
  (`PrimitiveComponent.SetSimulatePhysics` _mesh true)
  (`PrimitiveComponent.SetCollisionEnabled` _mesh "QueryAndPhysics")
  (`BrainComponent.StopLogic` (`AIController.BrainComponent` (`self.AICEnemyBase`)) "")
  (`/Game/Drkong/Enemy/AI/AIC_Enemy_Base.SetStateAsDead` (`self.AICEnemyBase`))
  (`SceneComponent.SetVisibility` (`self.HealthBar`) false true)
  (`KismetSystemLibrary.Delay` 3.0)
  (`self.K2_DestroyActor`))

(fn `GetCurrentHealth`
  (returns (Health :type "Float (double-precision)"))
  (return (`/Game/Drkong/DamageSystem/BPC_DamageSystem.Health` (`self.BPC_DamageSystem`))))

(fn `GetIdealRange`
  (returns (AttackRadius :type "Float (double-precision)"))
  (return 150.0))

(fn `GetMaxHealth`
  (returns (MaxHealth :type "Float (double-precision)"))
  (return (`/Game/Drkong/DamageSystem/BPC_DamageSystem.MaxHealth` (`self.BPC_DamageSystem`))))

(fn `Heal`
  (params (Amount :type "Float (double-precision)"))
  (returns (NewHealth :type "Float (double-precision)"))
  (return 0.0))

(fn `IsDead`
  (returns (Dead :type Boolean))
  (return false))

(fn `SetMovementSpeed`
  (params (Speed :type "/Game/Drkong/Enemy/AI/Enums/E_MovementSpeed Enum" :default "NewEnumerator0"))
  (returns (SpeedValue :type "Float (double-precision)"))
  (bind _output_get (set `CharacterMovementComponent.MaxWalkSpeed` (select `/Game/Drkong/Enemy/AI/Enums/E_MovementSpeed` Speed :`NewEnumerator1` 100.0 :`NewEnumerator2` 500.0 :!type "Float (single-precision)") (`self.CharacterMovement`)))
  (return _output_get))

(fn `TakeDamage`
  (params (DamageInfo :type "/Game/Drkong/DamageSystem/S_DamageInfo Structure"))
  (returns (WasDamaged :type Boolean))
  (`/Game/Drkong/DamageSystem/BPC_DamageSystem.TakeDamage` (`self.BPC_DamageSystem`) DamageInfo)
  (return false))

(fn `UserConstructionScript`)