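; BP_AliesBase is a base Blueprint for AI-controlled allies.
; On BeginPlay it casts its AI controller to AIC_Alies_Base and caches the reference.
; Its functions for health, damage, healing, death checks, movement speed and ideal range are all stubs that return zero or false, with no logic of their own.
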(event `self.ReceiveBeginPlay`
  (bind _asaic_alies_base (cast `/Game/Drkong/Alies/AIC_Alies_Base` (`AIBlueprintHelperLibrary.GetAIController` self)))
  (set `self.AICAliesBase` _asaic_alies_base))

(fn `GetCurrentHealth`
  (returns (Health :type "Float (double-precision)"))
  (return 0.0))

(fn `GetIdealRange`
  (returns (AttackRadius :type "Float (double-precision)"))
  (return 0.0))

(fn `GetIdealRangeAlies`
  (returns (AttackRadius :type "Float (double-precision)"))
  (return 0.0))

(fn `GetMaxHealth`
  (returns (MaxHealth :type "Float (double-precision)"))
  (return 0.0))

(fn `Heal`
  (params (Amount :type "Float (double-precision)"))
  (returns (NewHealth :type "Float (double-precision)"))
  (return 0.0))

(fn `IsDead`
  (returns (Dead :type Boolean))
  (return false))

(fn `SetMovementSpeed`
  (params (Speed :type "/Game/Drkong/Enemy/AI/Enums/E_MovementSpeed Enum" :default "NewEnumerator0"))
  (returns (SpeedValue :type "Float (double-precision)"))
  (return 0.0))

(fn `TakeDamage`
  (params (DamageInfo :type "/Game/Drkong/DamageSystem/S_DamageInfo Structure"))
  (returns (WasDamaged :type Boolean))
  (return false))

(fn `UserConstructionScript`)