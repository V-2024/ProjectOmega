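; BP_Alies_Ranged is a ranged ally character on team 0 that fires rifle bullets and reports a long ideal attack range.
; DefaultAttack plays a sped-up rifle montage, whose notify spawns a projectile from the left-hand socket toward the target with slight random yaw spread.
; Projectile impact sends damage to the hit actor through a damage message.
; Montage completion or interruption signals the attack's end.
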(event `self.ReceiveBeginPlay`
  (`parent.ReceiveBeginPlay`))

(event `self.DefaultAttack`
  (params (AttackTarget :type "Actor Object Reference"))
  (set `self.Attack Target` AttackTarget)
  (bind _notifyname (`|PlayMontage` (`self.Mesh`) "/Game/Drkong/Enemy/Animations/Montage/Rifle_Attack_01.Rifle_Attack_01" 3.0)
    (:`OnCompleted`
      (`self.OnAttackEnd` :!label _label))
    (:`OnInterrupted`
      (goto _label))
    (:`OnNotifyBegin`
      (switch `name` _notifyname
        (:`Fire`
          (`/Engine/EditorBlueprintResources/StandardMacros.IsValid` (`self.Attack Target`)
            (:`Is Valid`
              (bind _returnvalue (`|SpawnActorFromClass` "/Game/Drkong/Projectiles/BP_ProjectileBullet.BP_ProjectileBullet_C" (`KismetMathLibrary.MakeTransform` (`SceneComponent.GetSocketLocation` (`self.Mesh`) "hand_l") (`KismetMathLibrary.ComposeRotators` (`KismetMathLibrary.FindLookAtRotation` (`self.K2_GetActorLocation`) (`self.K2_GetActorLocation` AttackTarget)) (`KismetMathLibrary.MakeRotator` 0.0 0.0 (`KismetMathLibrary.RandomFloatInRange` -3.0 3.0)))) "Undefined" "MultiplyWithRoot" self 6000.0 0.0 null false null))
              (add `/Game/Drkong/Projectiles/BP_Projectile_Base.OnProjectileImpact` _returnvalue (delegate `ProjectileDamage`))
              (`PrimitiveComponent.IgnoreActorWhenMoving` (`self.CapsuleComponent`) _returnvalue true))))))))

(event `ProjectileDamage`
  (params (OtherActor :type "Actor Object Reference") (Hit :type "HitResult Structure"))
  (message `/Game/Drkong/DamageSystem/BPI_Damageable.TakeDamage` OtherActor (make `/Game/Drkong/DamageSystem/S_DamageInfo` 1.0 "NewEnumerator2")))

(fn `GetIdealRange`
  (returns (AttackRadius :type "Float (double-precision)"))
  (return 2000.0))

(fn `GetTeamNumber`
  (returns (`Team Number` :type Integer))
  (return 0))

(fn `UserConstructionScript`
  (`parent.UserConstructionScript`))